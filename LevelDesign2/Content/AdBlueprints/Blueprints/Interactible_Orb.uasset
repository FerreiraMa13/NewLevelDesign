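; Interactible orb that becomes usable when triggered and toggles between dormant and active materials on each interaction.
; Tick ramps a particle spawn rate up to a maximum on activation, then down to zero after one-shot use, destroying the particles after a delay.
; With DoOnce set, interaction also disables the orb and calls Triggered on a linked actor through TriggerInterface, allowing chained triggers.
; Construction script sizes the trigger capsule.
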(event Custom|Light%20Up
  ;[1 1 1] Orb's Light
  (Rendering|Material|SetMaterial (Variables|Default|GetOrb%20%28Inward%29) 0 "/Game/ThirdPersonBP/Materials/Placeable_Orbs_Active.Placeable_Orbs_Active")
  (Variables|Default|SetOn true))

(event Custom|Light%20Off
  ;[1 1 1] Orb's Light
  (Rendering|Material|SetMaterial (Variables|Default|GetOrb%20%28Inward%29) 0 "/Game/ThirdPersonBP/Materials/Placeable_Orbs_Dormant.Placeable_Orbs_Dormant")
  (Variables|Default|SetOn false))

(event EventTriggered
  ;[1 1 1] Triggered
  (if (not (Variables|Default|GetInteractible))
    (Variables|Default|SetInteractible true)
    (Variables|Default|SetParticle%20Stable false)))

(event EventInteraction
  (bind _triggerable (Variables|Default|GetTriggerable))
  ;[1 1 1] Triggered / Interacted
  (if (Variables|Default|GetInteractible)
    (if (Variables|Default|GetOn)
      (CallFunction|LightOff)
      (else
        (CallFunction|LightUp)))
    (if (Variables|Default|GetDo%20Once)
      (Variables|Default|SetParticle%20Stable false)
      (Variables|Default|SetInteractible false)
      (if (Utilities|IsValid _triggerable)
        (if (Utilities|DoesObjectImplementInterface _triggerable "/Game/AdBlueprints/Blueprints/TriggerInterface.TriggerInterface_C")
          (bind _astrigger_interface (Utilities|Casting|CastToTriggerInterface (Variables|Default|GetTriggerable)))
          (Default|Triggered _astrigger_interface))))))

(event EventTick
  (params (DeltaSeconds :type Float%20%28single-precision%29))
  ;[1 1 1] Tick
  (Variables|Default|Setdt DeltaSeconds)
  (if (and (Variables|Default|GetInteractible) (not (Variables|Default|GetParticle%20Stable)))
    (if (not (Variables|Default|GetDecay))
      ;;[1 1 1] Spawn
      (bind _output_get (Variables|Default|SetParticle%20Rate (+ (Variables|Default|GetParticle%20Rate) (* (Variables|Default|Getdt) 3e+01))))
      (if (> _output_get (Variables|Default|GetParticle%20Max%20Rate))
        (Variables|Default|SetParticle%20Rate (Variables|Default|GetParticle%20Max%20Rate)))
      (Niagara|SetNiagaraVariable(Float) (Variables|Default|GetParticles) "CustomSpawnRate" (Variables|Default|GetParticle%20Rate))
      (if (== (Variables|Default|GetParticle%20Rate) (Variables|Default|GetParticle%20Max%20Rate))
        (Variables|Default|SetParticle%20Stable true)
        (Variables|Default|SetDecay true)))
    (elif (and (Variables|Default|GetDecay) (not (Variables|Default|GetParticle%20Stable)))
      ;;[1 1 1] Decay
      (bind _output_get_2 (Variables|Default|SetParticle%20Rate (- (Variables|Default|GetParticle%20Rate) (* (Variables|Default|Getdt) 3e+01))))
      (if (< _output_get_2 0.0)
        (Variables|Default|SetParticle%20Rate 0.0))
      (Niagara|SetNiagaraVariable(Float) (Variables|Default|GetParticles) "CustomSpawnRate" (Variables|Default|GetParticle%20Rate))
      (if (== (Variables|Default|GetParticle%20Rate) 0.0)
        (Variables|Default|SetParticle%20Stable true)
        (Utilities|FlowControl|Delay 3.0)
        (Components|DestroyComponent (Variables|Default|GetParticles))))))

(fn ConstructionScript
  (Components|Capsule|SetCapsuleHalfHeight (Variables|Default|GetTrigger) (Variables|Default|GetTrigger%20Height) true)
  (Components|Capsule|SetCapsuleRadius (Variables|Default|GetTrigger) (Variables|Default|GetTrigger%20Radius) true))