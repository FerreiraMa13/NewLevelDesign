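; Blueprint function library with FindNearestActorOfClass, which finds the closest actor of a given class to a starting point.
; It scans all actors of that class, keeping the smallest distance below a running local value.
; For Interactible, Valid instances take priority over nearer invalid ones, which compete only until a valid one is found.
; It returns the nearest actor, its distance and a flag marking whether a valid Interactible was found.
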(fn FindNearestActorOfClass
  (params (Class :type Actor%20Class%20Reference) (StartingPoint :type Vector))
  (if (== Class "/Game/AdBlueprints/Blueprints/Interactible.Interactible_C")
    (bind _outactors (Actor|GetAllActorsOfClass 0 Class))
    (for _array_element _outactors
      (bind _asinteractible (Utilities|Casting|CastToInteractible _array_element))
      (if (Variables|/Game/AdBlueprints/Blueprints/Interactible.Interactible_C|GetValid _asinteractible)
        (if (LocalVariables|GetEnabled?)
          ;[0.3 1 0.6] Compare Distances
          (if (< (Math|Vector|Distance(Vector) (Transformation|GetActorLocation _asinteractible) StartingPoint) (LocalVariables|GetLocalNearestDistance))
            ;[1 0.9 0.5] Set Values
            (LocalVariables|SetLocalNearestDistance (Math|Vector|Distance(Vector) (Transformation|GetActorLocation _asinteractible) StartingPoint) :!label _label)
            (LocalVariables|SetLocalNearestActor _asinteractible))
          (else
            ;[1 0.9 0.5] Set Values
            (LocalVariables|SetEnabled? true)
            (LocalVariables|SetLocalNearestDistance (Math|Vector|Distance(Vector) (Transformation|GetActorLocation _asinteractible) StartingPoint))
            (LocalVariables|SetLocalNearestActor _asinteractible)))
        (elif (not (LocalVariables|GetEnabled?))
          ;[0.3 1 0.6] Compare Distances
          (if (< (Math|Vector|Distance(Vector) (Transformation|GetActorLocation _asinteractible) StartingPoint) (LocalVariables|GetLocalNearestDistance))
            (goto _label)))))
    ;[0.1 0 0.2] Return
    (return (LocalVariables|GetLocalNearestActor) (LocalVariables|GetLocalNearestDistance) (LocalVariables|GetEnabled?))
    (else
      (bind _outactors_2 (Actor|GetAllActorsOfClass 0 Class))
      (for _array_element_2 _outactors_2
        ;[0.3 1 0.6] Compare Distances
        (if (< (Math|Vector|Distance(Vector) (Transformation|GetActorLocation _array_element_2) StartingPoint) (LocalVariables|GetLocalNearestDistance))
          ;[1 0.9 0.5] Set Values
          (LocalVariables|SetLocalNearestDistance (Math|Vector|Distance(Vector) (Transformation|GetActorLocation _array_element_2) StartingPoint))
          (LocalVariables|SetLocalNearestActor _array_element_2)))
      ;[0.1 0 0.2] Return
      (return (LocalVariables|GetLocalNearestActor) (LocalVariables|GetLocalNearestDistance) (LocalVariables|GetEnabled?)))))