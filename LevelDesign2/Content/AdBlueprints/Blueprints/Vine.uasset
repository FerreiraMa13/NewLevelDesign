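; Zipline-style vine that carries the player along a spline when interacted with; interacting again mid-ride stops it.
; The construction script fits the cable, capsule collision and spline mesh to the spline, aligns particles and derives timeline speed from TravelDuration.
; Interaction seeds the Travel timeline from the player's distance along the vine, choosing direction by facing versus the Arrow unless OneWay.
; The timeline moves the player each update and changes character State on finish.
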(event EventInteraction
  (bind _spline (Variables|Default|GetSpline))
  (if (Audio|Components|Audio|IsPlaying (Variables|Default|GetTravel))
    ;[1 1 1] Zip
    (bind _traveldistance (Timeline|Travel Stop)
      (:Update
        (Transformation|SetActorLocation (Game|GetPlayerCharacter 0) (Math|Vector|MakeVector (.x (Spline|GetLocationatDistanceAlongSpline _spline (* _traveldistance (Spline|GetSplineLength _spline)) "World")) (.y (Spline|GetLocationatDistanceAlongSpline _spline (* _traveldistance (Spline|GetSplineLength _spline)) "World")) (+ (.z (Spline|GetLocationatDistanceAlongSpline _spline (* _traveldistance (Spline|GetSplineLength _spline)) "World")) 1e+02)) false false))
      (:Finished
        (bind _asthird_person_character (Utilities|Casting|CastToThirdPersonCharacter (Game|GetPlayerCharacter 0)))
        (Variables|/Game/AdBlueprints/Blueprints/ThirdPersonCharacter.ThirdPersonCharacter_C|SetState _asthird_person_character "NewEnumerator1")))
    (else
      (CallFunction|GetDistanceRatio)
      (bind _direction (CallFunction|DetectDirection))
      (if (Variables|Default|GetOne_way)
        (Timeline|Travel Play)
        (elif (>= _direction 0.0)
          (Timeline|Travel Play)
          (else
            (Timeline|Travel Reverse)))))))

(fn ConstructionScript
  (CallFunction|CableSetUp)
  (CallFunction|CollisionSetUp)
  (CallFunction|MeshSetUp)
  (Transformation|SetWorldRotation (Variables|Default|GetParticles) (Transformation|GetWorldRotation (Variables|Default|GetArrow)) false false)
  (Components|Timeline|SetPlayRate (Variables|Default|GetTravel) (/ 1.0 (Variables|Default|GetTravel%20Duration))))

(fn CableSetUp
  (bind _cable (Variables|Default|GetCable))
  (Transformation|SetWorldLocation (Variables|Default|GetCable) (Spline|GetLocationatSplinePoint (Variables|Default|GetSpline) 0 "World") false false)
  (Variables|/Script/CableComponent.CableComponent|SetbAttachEnd _cable true)
  (Variables|/Script/CableComponent.CableComponent|SetEndLocation _cable (Spline|GetLocationatSplinePoint (Variables|Default|GetSpline) 1 "Local"))
  (Variables|/Script/CableComponent.CableComponent|SetCableLength (Variables|Default|GetCable) (Spline|GetSplineLength (Variables|Default|GetSpline))))

(fn CollisionSetUp
  (bind _output_get (LocalVariables|SetSpline%20Half%20Lenght (* (Spline|GetSplineLength (Variables|Default|GetSpline)) 0.5)))
  (Components|Capsule|SetCapsuleRadius (Variables|Default|GetCollision) 125.0 true)
  (Components|Capsule|SetCapsuleHalfHeight (Variables|Default|GetCollision) _output_get true)
  (Transformation|SetWorldTransform (Variables|Default|GetCollision) (Math|Transform|MakeTransform (.location (Spline|GetTransformatDistanceAlongSpline (Variables|Default|GetSpline) _output_get "World" false)) (Math|Rotator|MakeRotator (.roll (.rotation (Spline|GetTransformatDistanceAlongSpline (Variables|Default|GetSpline) _output_get "World" false))) (+ (.pitch (.rotation (Spline|GetTransformatDistanceAlongSpline (Variables|Default|GetSpline) _output_get "World" false))) 9e+01) (.yaw (.rotation (Spline|GetTransformatDistanceAlongSpline (Variables|Default|GetSpline) _output_get "World" false)))) "1,1,1") false false))

(fn DetectDirection
  (return (Math|Vector|DotProduct (Math|Vector|GetForwardVector (Variables|/Script/Engine.Character|GetCapsuleComponent (Game|GetPlayerCharacter 0))) (Math|Vector|GetForwardVector (Transformation|GetWorldRotation (Variables|Default|GetArrow))))))

(fn GetDistanceRatio
  (bind _returnvalue (Game|GetPlayerCharacter 0))
  (bind _spline (Variables|Default|GetSpline))
  (bind _travel (Variables|Default|GetTravel))
  (bind _spline_2 (Variables|Default|GetSpline))
  (bind _returnvalue_2 (Transformation|GetActorLocation _returnvalue))
  (bind _returnvalue_3 (Spline|GetLocationatSplinePoint _spline 0 "World"))
  (bind _returnvalue_4 (Spline|GetSplineLength _spline_2))
  (bind _returnvalue_5 (Components|Timeline|GetTimelineLength _travel))
  (bind _returnvalue_6 (- _returnvalue_2 _returnvalue_3))
  (bind _returnvalue_7 (Math|Vector|VectorLength _returnvalue_6))
  (bind _returnvalue_8 (/ _returnvalue_7 _returnvalue_4))
  (bind _returnvalue_9 (* _returnvalue_5 _returnvalue_8))
  (Components|Timeline|SetNewTime _travel _returnvalue_9)
  (return _returnvalue_9))

(fn MeshSetUp
  (bind _spline (Variables|Default|GetSpline))
  (bind _splinemesh (Variables|Default|GetSplineMesh))
  (bind _splinemesh_2 (Variables|Default|GetSplineMesh))
  (bind (_location _tangent) (Spline|GetLocationandTangentatSplinePoint _spline 1 "Local"))
  (bind (_location_2 _tangent_2) (Spline|GetLocationandTangentatSplinePoint _spline 0 "Local"))
  (bind _relativelocation (Variables|/Script/Engine.SceneComponent|GetRelativeLocation _splinemesh_2))
  (SplineMesh|SetForwardAxis _splinemesh "Y" true)
  (SplineMesh|SetStartandEnd _splinemesh _location_2 _tangent_2 _location _tangent true :!class /Script/Engine.SplineMeshComponent)
  (Collision|SetCollisionEnabled _splinemesh "NoCollision")
  (Transformation|SetWorldScale3D _splinemesh_2 "0.200000,0.200000,0.200000")
  (Transformation|SetRelativeLocation _splinemesh_2 (Math|Vector|MakeVector (.x _relativelocation) (- (.y _relativelocation) (* 15.0 0.2)) (.z _relativelocation)) false false))