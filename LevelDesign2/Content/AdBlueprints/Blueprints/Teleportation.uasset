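; Teleporter actor that moves the player character to its Sphere's location when the player enters its Trigger, ignoring overlaps from the character's InteractionRadius.
; The player lands slightly below the Sphere's center, with movement stopped and the mode set to Falling.
; When FogTrigger is set, the teleport also flips the fogs through FogManager.
; The construction script disables Sphere collision, leaving it as a destination marker.
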(event OnComponentBeginOverlap(Trigger)
  (params (OverlappedComponent :type Primitive%20Component%20Object%20Reference) (OtherActor :type Actor%20Object%20Reference) (OtherComp :type Primitive%20Component%20Object%20Reference) (OtherBodyIndex :type Integer) (bFromSweep :type Boolean) (SweepResult :type Hit%20Result%20Structure%20%28by%20ref%29))
  (bind _returnvalue (Game|GetPlayerCharacter 0))
  (bind _returnvalue_2 (Game|GetPlayerCharacter 0))
  (bind _sphere (Variables|Default|GetSphere))
  (bind _returnvalue_3 (Transformation|GetWorldLocation _sphere))
  (bind _charactermovement (Variables|/Script/Engine.Character|GetCharacterMovement _returnvalue_2))
  (bind _asthird_person_character (Utilities|Casting|CastToThirdPersonCharacter _returnvalue))
  (if (and (!= OtherComp (Variables|/Game/AdBlueprints/Blueprints/ThirdPersonCharacter.ThirdPersonCharacter_C|GetInteraction%20Radius _asthird_person_character)) (== OtherActor _returnvalue))
    (Transformation|SetActorLocation _returnvalue_2 (Math|Vector|MakeVector (.x _returnvalue_3) (.y _returnvalue_3) (- (.z _returnvalue_3) 1e+01)) false true)
    (Components|Movement|StopMovementImmediately _charactermovement)
    (Pawn|Components|CharacterMovement|SetMovementMode _charactermovement "MOVE_Falling" 0)
    (if (Variables|Default|GetFog%20Trigger)
      (Default|FlipFogs (Variables|Default|GetFog%20Manager)))))

(fn ConstructionScript
  (Collision|SetCollisionEnabled (Variables|Default|GetSphere) "NoCollision"))