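; Spire landing point that pulls the player onto a spire when interacted with while high enough relative to its base.
; Interaction inserts a temporary spline point just above the player's mesh, forming a jump path.
; The PlayerJump timeline plays in reverse to move the player along that spline toward its start.
; On landing, it removes the point and advances the character's state if it matches a specific value.
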(event EventInteraction
  (bind _spline (Variables|Default|GetSpline))
  (if (not (Audio|Components|Audio|IsPlaying (Variables|Default|GetPlayer%20Jump)))
    (if (> (.z (Transformation|GetActorLocation (Game|GetPlayerCharacter 0))) (- (.z (Transformation|GetWorldLocation (Variables|Default|GetSpire%20Base))) (Variables|Default|GetZ_Margin)))
      (CallFunction|SplineSetUp)
      (bind _distance (Timeline|Player%20Jump ReverseFromEnd)
        (:Update
          ;[1 1 1] Jump To Spire
          (Transformation|SetActorLocation (Game|GetPlayerCharacter 0) (Spline|GetLocationatDistanceAlongSpline _spline (* _distance (Spline|GetSplineLength _spline)) "World") false false))
        (:Finished
          ;[1 1 1] Land
          (CallFunction|SplineReset)
          (bind _asthird_person_character (Utilities|Casting|CastToThirdPersonCharacter (Game|GetPlayerCharacter 0)))
          (if (Utilities|Enum|Equal(Enum) (Variables|/Game/AdBlueprints/Blueprints/ThirdPersonCharacter.ThirdPersonCharacter_C|GetState _asthird_person_character) "NewEnumerator2")
            (Variables|/Game/AdBlueprints/Blueprints/ThirdPersonCharacter.ThirdPersonCharacter_C|SetState _asthird_person_character "NewEnumerator3")))))))

(fn ConstructionScript)

(fn SplineSetUp
  (bind _returnvalue (Game|GetPlayerCharacter 0))
  (bind _mesh (Variables|/Script/Engine.Character|GetMesh _returnvalue))
  (bind _returnvalue_2 (Transformation|GetWorldLocation _mesh))
  (Spline|AddSplinePointatIndex (Variables|Default|GetSpline) (Math|Vector|MakeVector (.x _returnvalue_2) (.y _returnvalue_2) (+ (.z _returnvalue_2) 1e+02)) 1 "World" true))

(fn SplineReset
  (Spline|RemoveSplinePoint (Variables|Default|GetSpline) 1 true))