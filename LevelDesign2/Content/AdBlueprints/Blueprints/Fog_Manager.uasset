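; Fog manager Blueprint that switches between cavern and pit lighting setups by changing the visibility of two fogs and two skylights.
; The Triggered event hides CavernFog and Skylight1, then shows PitFog and Skylight2, propagating the fog changes to children.
; FlipFogs toggles both fogs relative to their current state without propagation, but always turns Skylight1 on and Skylight2 off.
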(event EventTriggered
  (Rendering|SetVisibility (Variables|Default|GetCavern%20Fog) false true)
  (Rendering|SetVisibility (Variables|Default|GetPit%20Fog) true true)
  (Rendering|SetVisibility (Variables|/Script/Engine.SkyLight|GetLightComponent (Variables|Default|GetSkylight%201)) false false)
  (Rendering|SetVisibility (Variables|/Script/Engine.SkyLight|GetLightComponent (Variables|Default|GetSkylight%202)) true false))

(fn ConstructionScript)

(fn FlipFogs
  (Rendering|ToggleVisibility (Variables|Default|GetCavern%20Fog) false)
  (Rendering|ToggleVisibility (Variables|Default|GetPit%20Fog) false)
  (Rendering|SetVisibility (Variables|/Script/Engine.SkyLight|GetLightComponent (Variables|Default|GetSkylight%201)) true false)
  (Rendering|SetVisibility (Variables|/Script/Engine.SkyLight|GetLightComponent (Variables|Default|GetSkylight%202)) false false))