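; Pairing_Trigger is an interactable that, while active and paired, signals its partner through TriggerInterface when used.
; It then deactivates once, removes its meshes and light, messages three trails and fires an optional other trigger.
; Tick ramps the particle spawn rate down to zero, then destroys the particles after a short delay.
; The construction script derives the paired state from whether a partner is assigned and marks it accessible.
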(event EventTick
  (params (DeltaSeconds :type Float%20%28single-precision%29))
  ;[1 1 1] Tick
  (if (Variables|Default|GetDecay)
    (bind _output_get (Variables|Default|SetDecay_rate (- (Variables|Default|GetDecay_rate) (* DeltaSeconds 45.0))))
    (if (< _output_get 0.0)
      (Variables|Default|SetDecay_rate 0.0)
      (Variables|Default|SetDecay false))
    (Niagara|SetNiagaraVariable(Float) (Variables|Default|GetParticles) "CustomSpawnRate" _output_get)
    (elif (== (Variables|Default|GetDecay_rate) 0.0)
      (Variables|Default|SetDecay_rate -1.0)
      (Utilities|FlowControl|Delay 2.0)
      (Components|DestroyComponent (Variables|Default|GetParticles)))))

(event EventInteraction
  (bind _pair_partner (Variables|Default|GetPair%20Partner))
  ;[1 1 1] Interaction
  (if (Variables|Default|GetActive)
    (if (Variables|Default|GetPaired)
      (if (Utilities|DoesObjectImplementInterface _pair_partner "/Game/AdBlueprints/Blueprints/TriggerInterface.TriggerInterface_C")
        (Class|TriggerInterface|Triggered(Message) _pair_partner)
        (if (Variables|Default|GetDo_Once)
          (Variables|Default|SetActive false)
          (Variables|Default|SetDecay true)
          (Components|DestroyComponent (Variables|Default|GetStaticMesh1))
          (Components|DestroyComponent (Variables|Default|GetStaticMesh))
          (Components|DestroyComponent (Variables|Default|GetPointLight))
          (Class|TriggerInterface|Triggered(Message) (Variables|Default|GetTrail%201))
          (Class|TriggerInterface|Triggered(Message) (Variables|Default|GetTrail%202))
          (Class|TriggerInterface|Triggered(Message) (Variables|Default|GetTrail%203))
          (if (Utilities|IsValid (Variables|Default|GetOther%20Trigger))
            (if (Utilities|DoesObjectImplementInterface (Variables|Default|GetOther%20Trigger) "/Game/AdBlueprints/Blueprints/TriggerInterface.TriggerInterface_C")
              (bind _astrigger_interface (Utilities|Casting|CastToTriggerInterface (Variables|Default|GetOther%20Trigger)))
              (Default|Triggered _astrigger_interface))))))))

(fn ConstructionScript
  (|CallParentFunction)
  (Variables|Default|SetPaired (Utilities|IsValid (Variables|Default|GetPair%20Partner)))
  (Variables|Default|SetAccessible true))